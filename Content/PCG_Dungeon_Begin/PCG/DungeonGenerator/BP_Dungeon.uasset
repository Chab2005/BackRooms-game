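; Dungeon actor that post-processes PCG-generated room layouts once graph generation fires its external event.
; It first checks each BP_Room_Master's collision-zone boxes and destroys room actors they overlap.
; It then tests each room's cap collision boxes against end-arrow collision boxes, adding a child actor component at any box with no overlap to cap open ends.
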(event OnPCGGraphGeneratedExternal(PCG_Dungeon)
  (params (PCGComponent :type PCG%20Component%20Object%20Reference))
  (CallFunction|RoomOverlapCleanup)
  (CallFunction|SpawnRoomCaps))

(fn ConstructionScript)

(fn RoomOverlapCleanup
  (bind _outactors (Actor|GetAllActorsOfClass "/Game/PCG_Dungeon_Begin/Blueprints/DungeonRooms/BP_Room_Master.BP_Room_Master_C"))
  (for _array_element _outactors
    (for _array_element_2 (Components|GetChildrenComponents (Variables|/Game/PCG_Dungeon_Begin/Blueprints/DungeonRooms/BP_Room_Master.BP_Room_Master_C|GetCollisionZones_Grp _array_element) false)
      (bind _asbox_collision (Utilities|Casting|CastToBoxComponent _array_element_2))
      (bind (_outactors_2 _returnvalue) (Collision|ComponentOverlapActors _asbox_collision (Transformation|GetWorldTransform _asbox_collision) (Variables|Default|GetRoomColisions) "/Game/PCG_Dungeon_Begin/Blueprints/DungeonRooms/BP_Room_Master.BP_Room_Master_C"))
      (if _returnvalue
        (for _array_element_3 _outactors_2
          (Actor|DestroyActor _array_element_3))))))

(fn SpawnRoomCaps
  (bind _outactors (Actor|GetAllActorsOfClass "/Game/PCG_Dungeon_Begin/Blueprints/DungeonRooms/BP_Room_Master.BP_Room_Master_C"))
  (for _array_element _outactors
    (Variables|Default|SetCurrent%20Room _array_element)
    (for _array_element_2 (Components|GetChildrenComponents (Variables|/Game/PCG_Dungeon_Begin/Blueprints/DungeonRooms/BP_Room_Master.BP_Room_Master_C|GetRoomCapCollision_Grp _array_element) false)
      (bind _asbox_collision (Utilities|Casting|CastToBoxComponent _array_element_2))
      (bind _returnvalue (Class|KismetSystemLibrary|ComponentOverlapComponents _asbox_collision (Transformation|GetWorldTransform _asbox_collision) (Variables|Default|GetEnd%20Arrow%20Colision) "/Script/Engine.BoxComponent"))
      (if (not _returnvalue)
        (AddComponent|AddChildActorComponent (Variables|Default|GetCurrent%20Room) false (Transformation|GetRelativeTransform _asbox_collision))))))