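; BP_Room_Master is the base room Blueprint for a procedural dungeon, with a forward arrow, grouped end arrows and collision zones.
; Its construction script adds a child actor, apparently a player start, to a Starter-tagged room when no PlayerStart exists, and recolors that forward arrow.
; It then tags and hides end arrows, before a debug step marked for pre-shipping deletion re-shows them with the forward arrow and collision zones.
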(fn `AddEndArrowsExtras`
  (for _array_element (`SceneComponent.GetChildrenComponents` (`self.EndArrows_Grp`) false)
    (set `ActorComponent.ComponentTags` (`self.ArrowComponentTags`) _array_element)
    (`SceneComponent.SetVisibility` _array_element false false)))

(fn `Debugging (DeleteBeforeShipping)`
  (`SceneComponent.SetVisibility` (`self.Forward (local x+)`) true false)
  (for _array_element (`SceneComponent.GetChildrenComponents` (`self.EndArrows_Grp`) false)
    (`SceneComponent.SetVisibility` _array_element true false))
  (for _array_element_2 (`SceneComponent.GetChildrenComponents` (`self.CollisionZones_Grp`) false)
    (`SceneComponent.SetVisibility` _array_element_2 true false)))

(fn `SpawnPlayerStart`
  (if (`self.ActorHasTag` "Starter")
    (bind _outactors (`GameplayStatics.GetAllActorsOfClass` "/Script/Engine.PlayerStart"))
    (if (`KismetArrayLibrary.Array_IsEmpty` _outactors)
      (`AddComponent|NODE_AddChildActorComponent-0` :`self` self :`RelativeTransform` (`KismetMathLibrary.MakeTransform` (0.0 0.0 92.0)))
      (`ArrowComponent.SetArrowColor` (`self.Forward (local x+)`) (struct :`G` 1.0 :`B` 1.0 :`A` 1.0)))))

(fn `UserConstructionScript`
  (`|ExecutionSequence`
    (:`then_0`
      (`self.SpawnPlayerStart`))
    (:`then_1`
      (`self.AddEndArrowsExtras`))
    (:`then_2`
      (`self.Debugging (DeleteBeforeShipping)`))))